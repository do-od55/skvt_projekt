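; BP_SkvtPlayerController is the player controller that sets up input and HUD and lets the player swap between pawns.
; On BeginPlay, if the Enhanced Input subsystem is valid, it adds the PMI_SkvtMapping config and creates the WBP_PlayerHUD widget.
; IA_Swap gathers every Pawn in the world and possesses the one after the controlled pawn, wrapping to the first.
; CreateMainMenu is an empty stub.
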(event `self.ReceiveBeginPlay`
  (bind _returnvalue (pcsubsystem `EnhancedInputLocalPlayerSubsystem` self))
  (`/Engine/EditorBlueprintResources/StandardMacros.IsValid` _returnvalue
    (:`Is Valid`
      (`EnhancedInputSubsystemInterface.AddPlayerMappableConfig` _returnvalue "/Game/Skvt/Characters/Input/PMI_SkvtMapping.PMI_SkvtMapping" (struct))
      (`self.CreatePlayerHUD`))))

(event `EnhancedInput|/Game/Skvt/Characters/Input/Actions/IA_Swap`
  (params (ActionValue :type Boolean) (ElapsedSeconds :type "Float (double-precision)") (TriggeredSeconds :type "Float (double-precision)") (InputAction :type "InputAction Object Reference" :default "/Game/Skvt/Characters/Input/Actions/IA_Swap.IA_Swap"))
  (:`Triggered`
    (bind _outactors (`GameplayStatics.GetAllActorsOfClass` "/Script/Engine.Pawn"))
    (`self.Possess` (`self.Get Pawn To Possess` _outactors))))

(fn `CreateMainMenu`)

(fn `CreatePlayerHUD`
  (bind _returnvalue (`|CreateWidget` "/Game/Skvt/UI/Widgets/PlayerHUD/WBP_PlayerHUD.WBP_PlayerHUD_C" self))
  (bind _output_get (set `self.HUDWidget` _returnvalue))
  (`UserWidget.AddToViewport` _output_get 0))

(fn `Get Pawn To Possess`
  (params (`Pawn Array` :type "Array of Pawn Object Reference (by ref)"))
  (returns (`Selected Pawn` :type "Pawn Object Reference"))
  (bind _returnvalue (+ (`KismetArrayLibrary.Array_Find` `Pawn Array` (`self.K2_GetPawn`)) 1))
  (if (`KismetArrayLibrary.Array_IsValidIndex` `Pawn Array` _returnvalue)
    (return (`|GetArrayItem` `Pawn Array` _returnvalue))
    (else
      (return (`|GetArrayItem` `Pawn Array`)))))

(fn `UserConstructionScript`)