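; BP_SkvtGameMode is the game mode for Skvt, handling the handover of player control to another living character.
; On BeginPlay it caches the first player controller as a BP_SkvtPlayerController.
; PossessNextCharacter has that controller possess the result of FindNextCharacter, provided it is valid.
; FindNextCharacter searches all BP_SkvtBaseChar actors and returns the first one that is not dead, with no other ordering.
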(event `self.ReceiveBeginPlay`
  (bind _asbp_skvt_player_controller (cast `/Game/Skvt/Characters/BP_SkvtPlayerController` (`GameplayStatics.GetPlayerController` 0)))
  (set `self.ControllerRef` _asbp_skvt_player_controller))

(event `PossessNextCharacter`
  (bind _newparn (`self.FindNextCharacter`))
  (`/Engine/EditorBlueprintResources/StandardMacros.IsValid` _newparn
    (:`Is Valid`
      (`Controller.Possess` (`self.ControllerRef`) _newparn))))

(fn `FindNextCharacter`
  (returns (NewParn :type "Pawn Object Reference"))
  (bind _outactors (`GameplayStatics.GetAllActorsOfClass` "/Game/Skvt/Characters/BP_SkvtBaseChar.BP_SkvtBaseChar_C"))
  (for _array_element _outactors
    (if (not (`/Game/Skvt/Characters/BP_SkvtBaseChar.IsDead` _array_element))
      (return _array_element))))

(fn `UserConstructionScript`)